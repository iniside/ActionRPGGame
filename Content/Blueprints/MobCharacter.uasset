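; MobCharacter is an enemy character with a heart mesh that attacks player actors through gameplay effects.
; BeginPlay assigns a dynamic master material to the body mesh and plays a timeline that moves the heart, scaled by JumpHeight.
; AttackPlayer waits briefly, applies InstantEffect to the valid target and spawns a hit particle; destruction spawns a death particle.
; Self-protection and enemy-count decrement logic are present but disconnected.
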(event Custom|Attack%20Player
  (params (Player%20To%20Attack :type Actor%20Object%20Reference))
  (bind _self self)
  (Utilities|IsValid Player%20To%20Attack
    (:Is%20Valid
      (Utilities|FlowControl|Delay 0.8)
      (Development|PrintString (Utilities|String|BuildString(Object) "Attacking:: " "" Player%20To%20Attack))
      (Class|GABlueprintLibrary|ApplyEffectActor Player%20To%20Attack _self _self (Variables|Default|GetInstantEffect))
      (Effects|SpawnEmitteratLocation "/Game/SharedAssets/GameJam/Particles/P_HeartAttackPlayer.P_HeartAttackPlayer" (+ (Transformation|GetActorLocation Player%20To%20Attack) "0, 0,70.000000")))))

(event Custom|RepeatTimeline)

(event EventBeginPlay
  (bind _returnvalue (Rendering|Material|CreateDynamicMaterialInstance "/Game/SharedAssets/CharacterMaterials/M_CharacterMaster.M_CharacterMaster" :!class /Script/Engine.KismetMaterialLibrary))
  (Rendering|Material|SetMaterial (Variables|Character|GetMesh) 0 _returnvalue)
  (bind _newtrack_0 (Timeline|Timeline_1 Play)
    (:Update
      (Transformation|SetRelativeLocation (Variables|Default|GetHeartMesh) (* _newtrack_0 (Variables|Default|GetJumpHeight)) false))))

(event EventActorBeginOverlap
  (params (OtherActor :type Actor%20Object%20Reference)))

(event EventTick
  (params (DeltaSeconds :type Float%20%28single-precision%29)))

(event EventAnyDamage
  (params (Damage :type Float%20%28single-precision%29) (DamageType :type Damage%20Type%20Object%20Reference) (InstigatedBy :type Controller%20Object%20Reference) (DamageCauser :type Actor%20Object%20Reference)))

(event EventDestroyed
  (Effects|SpawnEmitteratLocation "/Game/SharedAssets/GameJam/Particles/P_HeartDeath.P_HeartDeath" (+ (Transformation|GetActorLocation) "0, 0,70.000000")))

(fn ConstructionScript)