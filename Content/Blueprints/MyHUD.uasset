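; MyHUD is a HUD Blueprint that draws a crosshair at the point where the player's ARCharacter is aiming.
; Each DrawHUD traces from the mesh's TraceSocket along the base aim rotation, ignoring the character.
; It centers the crosshair material on the projected hit location, or on screen center without a hit.
; A second trace with fewer object types only draws a one-frame debug line.
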(event EventDrawHUD
  (params (SizeX :type Integer) (SizeY :type Integer))
  (Variables|Default|SetHalfScreenX (* SizeX 0.5))
  (Variables|Default|SetHalfScreenY (* SizeY 0.5))
  (bind _asarcharacter (Utilities|Casting|CastToARCharacter (Game|GetPlayerCharacter 0)))
  (bind _outhit (Collision|LineTraceForObjects (Transformation|GetSocketLocation (Variables|/Script/Engine.Character|GetMesh _asarcharacter) "TraceSocket") (+ (Transformation|GetSocketLocation (Variables|/Script/Engine.Character|GetMesh _asarcharacter) "TraceSocket") (* (Math|Vector|GetForwardVector (Pawn|GetBaseAimRotation _asarcharacter)) 2e+04)) (Utilities|Array|MakeArray "ObjectTypeQuery1" "ObjectTypeQuery3" "ObjectTypeQuery2" "ObjectTypeQuery8") false (Utilities|Array|MakeArray _asarcharacter) "None"))
  (Collision|LineTraceForObjects (Transformation|GetSocketLocation (Variables|/Script/Engine.Character|GetMesh _asarcharacter) "TraceSocket") (+ (Transformation|GetSocketLocation (Variables|/Script/Engine.Character|GetMesh _asarcharacter) "TraceSocket") (* (Math|Vector|GetForwardVector (Pawn|GetBaseAimRotation _asarcharacter)) 2e+04)) (Utilities|Array|MakeArray "ObjectTypeQuery1" "ObjectTypeQuery3" "ObjectTypeQuery2") false (Utilities|Array|MakeArray _asarcharacter) "ForOneFrame")
  (if (.bBlockingHit (Collision|BreakHitResult _outhit))
    (Class|HUD|DrawMaterialSimple "/Game/ContentPacks/Crosshair2_Mat.Crosshair2_Mat" (- (.X (Math|Vector|BreakVector (Class|HUD|Project (.Location (Collision|BreakHitResult _outhit))))) 24.0) (- (.Y (Math|Vector|BreakVector (Class|HUD|Project (.Location (Collision|BreakHitResult _outhit))))) 24.0) 48.0 48.0 1.0 false)
    (else
      (Class|HUD|DrawMaterialSimple "/Game/ContentPacks/Crosshair2_Mat.Crosshair2_Mat" (- (Variables|Default|GetHalfScreenX) 24.0) (- (Variables|Default|GetHalfScreenY) 24.0) 48.0 48.0 1.0 false))))

(fn ConstructionScript)