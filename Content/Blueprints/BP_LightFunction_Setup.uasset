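; Light function setup Blueprint that aligns a directional light with the actor's rotation and drives shared lighting material parameters.
; When enabled, the construction script rotates the light and writes light function scale, offset and brightness limits to MP_LightingSetup as preview parameters.
; It also passes the actor's forward vector to MPC_MacroVariation as LightVector.
; UpdateLocalValues and DisableSelf are empty.
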(fn ConstructionScript
  (bind _returnvalue (Transformation|GetActorRotation))
  (if (Variables|Default|GetEnabled)
    (Transformation|SetWorldRotation (Variables|Default|GetDirectionalLight) _returnvalue false)
    (Variables|Default|SetLight%20Rotation _returnvalue)
    ;[1 1 1] Preview Params
    (Rendering|Material|SetScalarParameterValue "/Game/KiteDemo/Environments/ParameterCollections/MP_LightingSetup.MP_LightingSetup" "LightFunction Scale" (Variables|LightFunction|GetLF%20Scale) :!class /Script/Engine.KismetMaterialLibrary)
    (Rendering|Material|SetScalarParameterValue "/Game/KiteDemo/Environments/ParameterCollections/MP_LightingSetup.MP_LightingSetup" "LightFunction Offset" (Variables|LightFunction|GetLF%20Offset) :!class /Script/Engine.KismetMaterialLibrary)
    (Rendering|Material|SetScalarParameterValue "/Game/KiteDemo/Environments/ParameterCollections/MP_LightingSetup.MP_LightingSetup" "LightFunction Min" (Variables|LightFunction|GetLF%20Min%20Brightness) :!class /Script/Engine.KismetMaterialLibrary)
    (Rendering|Material|SetScalarParameterValue "/Game/KiteDemo/Environments/ParameterCollections/MP_LightingSetup.MP_LightingSetup" "LightFunction Max" (Variables|LightFunction|GetLF%20Max%20Brightness) :!class /Script/Engine.KismetMaterialLibrary)
    (Rendering|Material|SetVectorParameterValue "/Game/KiteDemo/Environments/ParameterCollections/MPC_MacroVariation.MPC_MacroVariation" "LightVector" (Math|Conversions|ToLinearColor(Vector) (Math|Rotator|GetRotationXVector _returnvalue)) :!class /Script/Engine.KismetMaterialLibrary)))

(fn UpdateLocalValues)

(fn DisableSelf)