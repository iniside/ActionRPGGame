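; AoEDummy is a character test dummy for gameplay effects, with nearly all of its logic disconnected.
; Its events and construction script are empty, leaving unwired chains for self-applied effects, heart animation, delayed player attacks, death particles and enemy-count decrement.
; ApplyEffectTimer applies a no-damage instant effect to the player character, but the looping timer that calls it sits in an unwired chain.
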(event Custom|Attack%20Player
  (params (Player%20To%20Attack :type Actor%20Object%20Reference)))

(event Custom|RepeatTimeline)

(event EventBeginPlay)

(event EventActorBeginOverlap
  (params (OtherActor :type Actor%20Object%20Reference)))

(event EventTick
  (params (DeltaSeconds :type Float%20%28single-precision%29)))

(event EventAnyDamage
  (params (Damage :type Float%20%28single-precision%29) (DamageType :type Damage%20Type%20Object%20Reference) (InstigatedBy :type Controller%20Object%20Reference) (DamageCauser :type Actor%20Object%20Reference)))

(event EventDestroyed)

(fn ConstructionScript)

(fn ApplyEffectTimer
  (bind _self self)
  (Class|GABlueprintLibrary|ApplyEffectActor (Game|GetPlayerCharacter 0) _self _self (Variables|Default|GetInstantEffectNoDamage)))