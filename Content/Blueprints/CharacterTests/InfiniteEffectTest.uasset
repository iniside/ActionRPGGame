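; Test character for gameplay effects, with a bobbing heart mesh and a heart particle burst when destroyed.
; BeginPlay applies a protection effect to itself, then loops through test effect specs, applying each.
; The same loop starts a randomly timed repeating timer that applies a no-damage instant effect to the player, sets a dynamic material and plays the bob timeline.
; Attack and enemy-count logic is left unwired.
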(event Custom|Attack%20Player
  (params (Player%20To%20Attack :type Actor%20Object%20Reference)))

(event Custom|RepeatTimeline)

(event EventBeginPlay
  (bind _self self)
  (bind _self_2 self)
  (Class|GAAttributeComponent|ApplySelfEffect _self _self _self (Variables|Default|GetProtectionEffect))
  (for _array_element (Variables|Default|GetEffectSpecsTest)
    (Class|GAAttributeComponent|ApplySelfEffect (Variables|Default|GetAttributes) _self_2 _self_2 _self_2 _array_element)
    (Utilities|Time|SetTimerbyFunctionName self "ApplyEffectTimer" (Math|Random|RandomFloatinRange 5.0 15.0) true)
    (bind _returnvalue (Rendering|Material|CreateDynamicMaterialInstance "/Game/SharedAssets/CharacterMaterials/M_CharacterMaster.M_CharacterMaster" :!class /Script/Engine.KismetMaterialLibrary))
    (Rendering|Material|SetMaterial (Variables|Character|GetMesh) 0 _returnvalue)
    (bind _newtrack_0 (Timeline|Timeline_1 Play)
      (:Update
        (Transformation|SetRelativeLocation (Variables|Default|GetHeartMesh) (* _newtrack_0 (Variables|Default|GetJumpHeight)) false)))))

(event EventActorBeginOverlap
  (params (OtherActor :type Actor%20Object%20Reference)))

(event EventTick
  (params (DeltaSeconds :type Float%20%28single-precision%29)))

(event EventAnyDamage
  (params (Damage :type Float%20%28single-precision%29) (DamageType :type Damage%20Type%20Object%20Reference) (InstigatedBy :type Controller%20Object%20Reference) (DamageCauser :type Actor%20Object%20Reference)))

(event EventDestroyed
  (Effects|SpawnEmitteratLocation "/Game/SharedAssets/GameJam/Particles/P_HeartDeath.P_HeartDeath" (+ (Transformation|GetActorLocation) "0, 0,70.000000")))

(fn ConstructionScript)

(fn ApplyEffectTimer
  (bind _self self)
  (Class|GABlueprintLibrary|ApplyEffectActor (Game|GetPlayerCharacter 0) _self _self (Variables|Default|GetInstantEffectNoDamage)))