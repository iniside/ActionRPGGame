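; Test character Blueprint that applies a ReduceOutgoingDamage effect to itself on BeginPlay, despite its SimpleNoEffects name.
; That effect application is its only live logic; the death handler is empty.
; Disconnected leftover graphs hold other self-effects, death cleanup, HUD widget creation, mob counting, and health bar updates that find the enemy by camera line trace.
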(event EventOnCharacterDied)

(event EventBeginPlay
  (bind _self self)
  (Class|GABlueprintLibrary|ApplyEffectActor _self _self _self (Variables|Default|GetReduceOutgoingDamage)))

(event EventActorBeginOverlap
  (params (OtherActor :type Actor%20Object%20Reference)))

(event Input|KeyboardEvents|M)

(fn ConstructionScript)