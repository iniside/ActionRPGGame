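; Cinematic spawner actor that places a group of deer within a radius and plays a montage on them.
; SpawnDeer traces down for ground height and spawns with varied yaw, using a random stream seeded from actor location in the construction script.
; Each deer has crowd steering suspended, registers with FlockManager and passes the manager and montage to its anim blueprint.
; KillDeer unregisters and destroys all spawned deer.
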(event Custom|SpawnDeer
  (bind _returnvalue (Transformation|GetActorLocation))
  (bind _returnvalue_2 (Transformation|GetActorRotation))
  (bind _spawnradius (Variables|Default|GetSpawnRadius))
  (bind _randomstream (Variables|Default|GetRandomStream))
  (bind (_pitch _yaw _roll) (Class|KismetMathLibrary|BreakRot _returnvalue_2))
  (bind _returnvalue_3 (Math|Random|RandomFloatinRangefromStream 0.0 _spawnradius _randomstream))
  (bind _returnvalue_4 (Math|Random|RandomFloatinRangefromStream 0.0 3.6e+02 _randomstream))
  (bind _returnvalue_5 (Math|Trig|Sin(Degrees) _returnvalue_4))
  (bind _returnvalue_6 (Math|Trig|Cos(Degrees) _returnvalue_4))
  (bind _returnvalue_7 (Math|Vector|MakeVector _returnvalue_5 _returnvalue_6 0.0))
  (bind _returnvalue_8 (* _returnvalue_7 _returnvalue_3))
  (bind _returnvalue_9 (+ _returnvalue_8 _returnvalue))
  ;[1 1 1] Spawn Deer
  (for _index (range 0 (- (Variables|Default|GetNumDeerToSpawn) 1))
    ;[1 1 1] Random location
    (bind _outhit (Collision|LineTraceByChannel (+ _returnvalue_9 "0, 0,1000.000000") (- _returnvalue_9 "0, 0,1000.000000") "TraceTypeQuery1" false 0 "None"))
    (bind _returnvalue_10 (Game|SpawnActorfromClass (Variables|Default|GetClassToSpawn) (Math|Transform|MakeTransform (+ (.Location (Collision|BreakHitResult _outhit)) "0, 0,88.000000") (Class|KismetMathLibrary|MakeRot _pitch (+ _yaw (Math|Random|RandomFloatinRangefromStream (* (Variables|Default|GetRotationVariance) -1.0) (Variables|Default|GetRotationVariance) _randomstream)) _roll)) false 0 0))
    (Utilities|Array|Add (Variables|Default|GetSpawnedDeer) _returnvalue_10)
    (bind _returnvalue_11 (AI|GetAIController _returnvalue_10))
    (bind _ascrowd_following_component (Utilities|Casting|CastToCrowdFollowingComponent (Class|AIController|GetPathFollowingComponent _returnvalue_11)))
    (Class|CrowdFollowingComponent|SuspendCrowdSteering _ascrowd_following_component true)
    (Class|FlockManager|TryRegisterAgent (Variables|Default|GetFlockManager) _returnvalue_10)
    (bind _asred_deer_anim_blueprint (Utilities|Casting|CastToRedDeerAnimBlueprint (Components|SkeletalMesh|GetAnimInstance (Variables|/Script/Engine.Character|GetMesh _returnvalue_10))))
    (Variables|/Game/Meshes/Deer/RedDeerAnimBlueprint.RedDeerAnimBlueprint_C|SetCinematicMontage _asred_deer_anim_blueprint (Variables|Default|GetCinematicMontage))
    (Variables|/Game/Meshes/Deer/RedDeerAnimBlueprint.RedDeerAnimBlueprint_C|SetFlockManager _asred_deer_anim_blueprint (Variables|Default|GetFlockManager))
    (Animation|Montage|MontagePlay (Components|SkeletalMesh|GetAnimInstance (Variables|/Script/Engine.Character|GetMesh _returnvalue_10)) (Variables|Default|GetCinematicMontage) 1.0)))

(event Custom|KillDeer
  (bind _spawneddeer (Variables|Default|GetSpawnedDeer))
  ;[1 1 1] Kill Deer
  (for _array_element _spawneddeer
    (Class|FlockManager|TryUnregisterAgent (Variables|Default|GetFlockManager) _array_element)
    (Actor|DestroyActor _array_element))
  (Utilities|Array|Clear _spawneddeer))

(fn ConstructionScript
  (bind _returnvalue (Transformation|GetActorLocation))
  (bind (_x _y _z) (Math|Vector|BreakVector _returnvalue))
  (Components|Sphere|SetSphereRadius (Variables|Default|GetSphere) (Variables|Default|GetSpawnRadius) true)
  (Math|Random|SetRandomStreamSeed (Variables|Default|GetRandomStream) (Math|Float|Floor (+ _x _y _z))))