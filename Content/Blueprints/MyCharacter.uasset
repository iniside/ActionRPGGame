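; Player character that serves as a test bed for inventory, action bar, looting and attribute components.
; BeginPlay builds an UberWidget hosting the inventory and loot widgets, while debug keys toggle inventory and action bar containers, add a test item and print attribute values.
; LootItem line-traces from the follow camera and passes any hit ARItemPickup to the inventory's GetLootContainer.
; Several disconnected leftover node chains never run.
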(event Custom|LootItem
  (bind _followcamera (Variables|Default|GetFollowCamera))
  (bind _returnvalue (Transformation|GetWorldLocation _followcamera))
  (bind _outhit (Collision|LineTraceByChannel _returnvalue (+ _returnvalue (* (Math|Vector|GetForwardVector (Transformation|GetWorldRotation _followcamera)) 1e+04)) "TraceTypeQuery1" false 0 "ForDuration"))
  (Utilities|IsValid (.HitActor (Collision|BreakHitResult _outhit))
    (:Is%20Valid
      (bind _asaritem_pickup (Utilities|Casting|CastToARItemPickup (.HitActor (Collision|BreakHitResult _outhit))))
      (Class|GISInventoryBaseComponent|GetLootContainer (Variables|Default|GetInventory) _asaritem_pickup)
      (Development|PrintString (Utilities|GetDisplayName (.HitActor (Collision|BreakHitResult _outhit)))))))

(event EventBeginPlay
  (bind _inventory (Variables|Default|GetInventory))
  (bind _returnvalue (UserInterface|CreateWidget "/Game/Blueprints/UberWidget.UberWidget_C"))
  (Variables|Default|SetUberWidget _returnvalue)
  (Widget|Panel|AddChild (Variables|/Game/Blueprints/UberWidget.UberWidget_C|GetInventoryBox (Variables|Default|GetUberWidget)) (Variables|/Script/GameInventorySystem.GISInventoryBaseComponent|GetInventoryContainer _inventory))
  (Widget|Panel|AddChild (Variables|/Game/Blueprints/UberWidget.UberWidget_C|GetLootingBox (Variables|Default|GetUberWidget)) (Variables|/Script/GameInventorySystem.GISInventoryBaseComponent|GetLootWidget _inventory))
  (UserInterface|Viewport|AddtoViewport (Variables|Default|GetUberWidget)))

(event Input|KeyboardEvents|F
  (:Pressed
    (UserInterface|Viewport|AddtoViewport (Variables|/Script/GameInventorySystem.GISInventoryBaseComponent|GetInventoryContainer (Variables|Default|GetInventory)))
    (UserInterface|Viewport|AddtoViewport (Variables|/Script/GameInventorySystem.GISInventoryBaseComponent|GetInventoryContainer (Variables|Default|GetActionBar)))))

(event Input|KeyboardEvents|G
  (:Pressed
    (bind _returnvalue (|CreateItemData "/GameInventorySystem/Test/TestItemData.TestItemData_C" (Game|GetPlayerController 0)))
    (Class|GISInventoryBaseComponent|AddItemtoInventory (Variables|Default|GetInventory) _returnvalue)))

(event Input|KeyboardEvents|Q
  (:Pressed
    (CallFunction|LootItem)))

(event Input|KeyboardEvents|E
  (:Pressed
    (bind _returnvalue (Class|GAAttributesBlueprintFunctionLibrary|GetAttribute "(AttributeName=\"Health\")"))
    (bind _returnvalue_2 (Class|GAAttributesBase|GetFloatValue (Variables|/Script/GameAttributes.GAAttributeComponent|GetDefaultAttributes (Variables|Default|GetAttributes)) "(AttributeName=\"Health\")"))
    (Development|PrintString (Utilities|String|BuildString(Float) (Utilities|String|ToString(Name) _returnvalue) "" _returnvalue_2))))

(event Input|KeyboardEvents|T
  (:Pressed
    (Widget|RemovefromParent (Variables|/Script/GameInventorySystem.GISInventoryBaseComponent|GetInventoryContainer (Variables|Default|GetInventory)))
    (Widget|RemovefromParent (Variables|/Script/GameInventorySystem.GISInventoryBaseComponent|GetInventoryContainer (Variables|Default|GetActionBar)))))

(event Input|KeyboardEvents|Z
  (:Pressed
    (bind _returnvalue (Class|GAAttributesBase|GetFloatValue (Variables|/Script/GameAttributes.GAAttributeComponent|GetDefaultAttributes (Variables|Default|GetAttributes)) "(AttributeName=\"Health\")"))
    (Development|PrintString (Utilities|String|BuildString(Float) (Utilities|String|ToString(Name) (stale Input|KeyboardEvents|E _returnvalue)) "" _returnvalue))))

(fn ConstructionScript)