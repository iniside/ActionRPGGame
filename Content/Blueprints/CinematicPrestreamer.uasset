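; CinematicPrestreamer is a Blueprint that controls level streaming, by its name to preload sublevels for cinematics.
; EnablePrestreaming toggles distance-based streaming on the KeepCurrentState and ForceToLoad levels.
; When enabled, it also forces ForceToLoad levels loaded and visible with blocking loads, then flushes level streaming.
; Disabling only restores distance streaming, without explicitly unloading anything.
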(fn ConstructionScript)

(fn EnablePrestreaming
  (params (bEnableParam :type Boolean :default false))
  (LocalVariables|SetEnable bEnableParam)
  (for _array_element (Variables|Default|GetKeepCurrentState)
    (Variables|/Script/Engine.LevelStreaming|SetbDisableDistanceStreaming (Class|GameplayStatics|GetStreamingLevel _array_element) (LocalVariables|GetEnable)))
  (if (LocalVariables|GetEnable)
    (for _array_element_2 (Variables|Default|GetForceToLoad)
      (Variables|/Script/Engine.LevelStreaming|SetbDisableDistanceStreaming (Class|GameplayStatics|GetStreamingLevel _array_element_2) true)
      (Variables|/Script/Engine.LevelStreaming|SetbShouldBeLoaded (Class|GameplayStatics|GetStreamingLevel _array_element_2) true)
      (Variables|/Script/Engine.LevelStreaming|SetbShouldBeVisible (Class|GameplayStatics|GetStreamingLevel _array_element_2) true)
      (Variables|/Script/Engine.LevelStreaming|SetbShouldBlockOnLoad (Class|GameplayStatics|GetStreamingLevel _array_element_2) true)
      (Variables|/Script/Engine.LevelStreaming|SetLevelLODIndex (Class|GameplayStatics|GetStreamingLevel _array_element_2) -1))
    (Class|GameplayStatics|FlushLevelStreaming)
    (else
      (for _array_element_3 (Variables|Default|GetForceToLoad)
        (Variables|/Script/Engine.LevelStreaming|SetbDisableDistanceStreaming (Class|GameplayStatics|GetStreamingLevel _array_element_3) false)))))