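; GES_DecreaseDamage is a test effect modifier that lowers the value of incoming effects.
; ModifyIncomingEffect casts the effect to GES_EffectTest, subtracts a fixed amount from its BaseValue in place, then prints the effect's target.
; ModifyOutgoingEffect only prints the target and leaves the effect unchanged.
; Both overrides return false, except that the incoming one stops early when the cast fails.
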(fn ModifyIncomingEffect
  (params (EffectIn :type GES%20Effect%20Object%20Reference))
  (bind _asges_effect_test (Utilities|Casting|CastToGES_EffectTest EffectIn))
  (Variables|/Game/Blueprints/Test/GES_EffectTest.GES_EffectTest_C|SetBaseValue _asges_effect_test (- (Variables|/Game/Blueprints/Test/GES_EffectTest.GES_EffectTest_C|GetBaseValue _asges_effect_test) 5.0))
  (Development|PrintString 0 (Utilities|String|BuildString(Object) "incoming::  " "" (Variables|/Script/GameEffectSystem.GESEffect|GetTarget EffectIn)))
  (return false))

(fn ModifyOutgoingEffect
  (params (EffectIn :type GES%20Effect%20Object%20Reference))
  (Development|PrintString 0 (Utilities|String|BuildString(Object) "Outgoing::  " "" (Variables|/Script/GameEffectSystem.GESEffect|GetTarget EffectIn)))
  (return false))