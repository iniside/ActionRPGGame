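; Test ability Blueprint that, on activation, applies an attribute modifier to whatever the owning ARCharacter's camera is aimed at.
; A long, debug-drawn object trace runs from the follow camera along its forward vector, against pawns and static and dynamic world objects.
; The hit actor receives a fixed-value modifier with the character as instigator, then its attribute is read back and printed as target health.
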(event EventOnAbilityActivated
  (bind _asarcharacter (Utilities|Casting|CastToARCharacter (Components|GetOwner)))
  (bind _outhit (Collision|LineTraceForObjects (Transformation|GetWorldLocation (Variables|/Script/ActionRPGGame.ARCharacter|GetFollowCamera _asarcharacter)) (+ (Transformation|GetWorldLocation (Variables|/Script/ActionRPGGame.ARCharacter|GetFollowCamera _asarcharacter)) (* (Math|Vector|GetForwardVector (Transformation|GetWorldRotation (Variables|/Script/ActionRPGGame.ARCharacter|GetFollowCamera _asarcharacter))) 1e+04)) (Utilities|Array|MakeArray "ObjectTypeQuery3" "ObjectTypeQuery1" "ObjectTypeQuery2") false 0 "ForDuration"))
  (Variables|Default|SetLocation (.ImpactPoint (Collision|BreakHitResult _outhit)))
  (Class|GAAttributesBlueprintFunctionLibrary|ModifyAttributes (Utilities|Array|MakeArray (Utilities|Struct|MakeGAAttributeModifier (.HitActor (Collision|BreakHitResult _outhit)) _asarcharacter "(AttributeName=\"Health\")" (.Location (Collision|BreakHitResult _outhit)) 1e+01)))
  (bind _returnvalue (Class|GAAttributesBlueprintFunctionLibrary|GetAttributeFloat (.HitActor (Collision|BreakHitResult _outhit)) "(AttributeName=\"Health\")"))
  (Development|PrintString (Utilities|String|BuildString(Float) "Target Health::  " "" _returnvalue)))

(fn ConstructionScript)